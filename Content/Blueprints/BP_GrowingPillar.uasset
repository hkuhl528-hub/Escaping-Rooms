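; BP_GrowingPillar is an actor that enlarges its Templatedetail component in random, timed steps after BeginPlay.
; A DoN node with a random limit gates a loop of random delay and Grow call, which adds a random amount to relative scale on all axes.
; After each step, a zero check on the DoN counter either enables query-and-physics collision or loops back into the gate.
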(event Custom|Grow
  (bind _template_detail (Variables|Default|Gettemplate-detail))
  (Transformation|SetRelativeScale3D _template_detail (+ (Variables|/Script/Engine.SceneComponent|GetRelativeScale3D _template_detail) (Math|Random|RandomFloatinRange 0.1 0.5))))

(event EventBeginPlay
  (bind _counter (Utilities|FlowControl|DoN (Math|Random|RandomIntegerinRange 1 7) :!label _label)
    (:Exit
      (Utilities|FlowControl|Delay (Math|Random|RandomFloatinRange 2.5 5.0))
      (CallFunction|Grow)
      (if (== _counter 0)
        (Collision|SetCollisionEnabled (Variables|Default|Gettemplate-detail) "QueryAndPhysics")
        (else
          (goto _label))))))

(fn ConstructionScript)